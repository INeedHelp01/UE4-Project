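; MySplinePlatform is a platform actor that starts moving its mesh along a spline at BeginPlay.
; The construction script applies a configurable static mesh and material to the platform.
; A timeline's SplineDistance value, multiplied by Rate and spline length, sets the distance sampled for the mesh's world location, without sweep.
; The branch condition is fixed true, so the timeline reverse path never runs.
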(event `Platform Start`
  (bind _spline (`self.Spline`))
  (if true
    (bind (_direction _spline_distance) (`Timeline|Motion Timeline` :!via `PlayFromStart` :!label _label)
      (:`Update`
        (`SceneComponent.K2_SetWorldLocation` (`self.Platform Mesh`) (`SplineComponent.GetLocationAtDistanceAlongSpline` _spline (* (`SplineComponent.GetSplineLength` _spline) (* _spline_distance (`self.Rate`))) "World") false false)
        (if true
          _)))
    (else
      (goto _label :!via `Reverse`))))

(event `self.ReceiveBeginPlay`
  (`self.Platform Start`))

(fn `UserConstructionScript`
  (bind _platform_mesh (`self.Platform Mesh`))
  (`StaticMeshComponent.SetStaticMesh` _platform_mesh (`self.Static Mesh`))
  (`PrimitiveComponent.SetMaterial` _platform_mesh 0 (`self.Material`)))