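; Coin pickup actor that awards a point when a ThirdPersonCharacter overlaps its box.
; On overlap it destroys itself, plays a 2D sound and increments Points on the game manager's health widget.
; A separate SetPoints function caps Points and updates the widget, or refills them and changes game state at zero.
; ResetGame moves the actor to the first found coin's location; BeginPlay's coin search result is unused.
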(event `self.ReceiveBeginPlay`
  (`GameplayStatics.GetAllActorsOfClass` "Coin_BP_C"))

(event `self.Box.OnComponentBeginOverlap`
  (params (OverlappedComponent :type "PrimitiveComponent Object Reference") (OtherActor :type "Actor Object Reference") (OtherComp :type "PrimitiveComponent Object Reference") (OtherBodyIndex :type Integer) (bFromSweep :type Boolean) (SweepResult :type "HitResult Structure (by ref)"))
  (cast `/Game/ThirdPersonBP/Blueprints/ThirdPersonCharacter` OtherActor)
  (`self.K2_DestroyActor`)
  (`GameplayStatics.PlaySound2D` "/Game/__MyContent/Audio/Coin_2.Coin_2" 1.0 1.0 0.0 null null)
  (bind _my_game_manager (`/Game/__MyContent/Blueprints/MyFunctionLibrary.Get My Game Manager`))
  (bind _widget_health (`/Game/__MyContent/Blueprints/MyGameManager.Widget Health` _my_game_manager))
  (set `/Game/__MyContent/UI/Widget_health.Points` (+ (`/Game/__MyContent/UI/Widget_health.Points` _widget_health) 1.0) _widget_health))

(fn `Reset Game`
  (bind _outactors (`GameplayStatics.GetAllActorsOfClass` "Coin_BP_C"))
  (`self.K2_SetActorLocation` (`self.K2_GetActorLocation` (`|GetArrayItem` _outactors))))

(fn `set Points`
  (params (`Set Points` :type "Float (double-precision)"))
  (bind _output_get (set `self.Points` `Set Points`))
  (if (> _output_get 100.0)
    (set `self.Points` 100.0))
  (if (<= _output_get 0.0)
    (set `self.Points` 100.0)
    (bind _my_game_manager (`/Game/__MyContent/Blueprints/MyFunctionLibrary.Get My Game Manager`))
    (`/Game/__MyContent/Blueprints/MyGameManager.Set State` _my_game_manager "NewEnumerator1")
    (else
      (bind _my_game_manager_2 (`/Game/__MyContent/Blueprints/MyFunctionLibrary.Get My Game Manager`))
      (set `/Game/__MyContent/UI/Widget_health.Points` (`self.Points`) (`/Game/__MyContent/Blueprints/MyGameManager.Widget Health` _my_game_manager_2)))))

(fn `Start`)

(fn `UserConstructionScript`)